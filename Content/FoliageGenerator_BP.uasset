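; Foliage generator actor that scatters instances of a chosen mesh over a rectangular area sized by its root's X and Y scale.
; The construction script clears the Foliage instanced mesh component and loops by Density times that scale area.
; Each pass runs a short, debug-drawn downward Visibility trace at a random offset, adding an instance at the hit location without checking for a hit.
; BeginPlay only reassigns the mesh.
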(event `self.ReceiveBeginPlay`
  (`StaticMeshComponent.SetStaticMesh` (`self.Foliage`) (`self.FoliageMesh`)))

(fn `UserConstructionScript`
  (bind (_returnvalue_x _returnvalue_y) (`KismetMathLibrary.BreakVector` (`SceneComponent.K2_GetComponentScale` (`self.DefaultSceneRoot`))))
  (bind _returnvalue (+ (`SceneComponent.K2_GetComponentLocation` (`self.DefaultSceneRoot`)) (`KismetMathLibrary.MakeVector` (* (`KismetMathLibrary.RandomFloatInRange` 0.0 _returnvalue_x) 100.0) (* (`KismetMathLibrary.RandomFloatInRange` 0.0 _returnvalue_y) 100.0))))
  (`StaticMeshComponent.SetStaticMesh` (`self.Foliage`) (`self.FoliageMesh`))
  (`InstancedStaticMeshComponent.ClearInstances` (`self.Foliage`))
  (for _ (range (+ (`KismetMathLibrary.Round` (* (`self.Density`) _returnvalue_x _returnvalue_y)) 1))
    (bind _outhit (`KismetSystemLibrary.LineTraceSingle` :`Start` _returnvalue :`End` (- _returnvalue (0.0 0.0 50.0)) :`TraceChannel` "TraceTypeQuery1" :`DrawDebugType` "ForDuration" :`DrawTime` 0.6))
    (`InstancedStaticMeshComponent.AddInstance` (`self.Foliage`) (`KismetMathLibrary.Conv_VectorToTransform` (`.Location` (`GameplayStatics.BreakHitResult` _outhit))) true)))